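; BP_Repeater is a construction-time tool that repeats one static mesh in a straight, evenly spaced line.
; Its construction script fills an InstancedStaticMesh with Count instances, each stepped by a multiple of Offset from one Offset onward, sharing Rotation and Scale.
; The rebuild runs only when Count differs from the cached MaxCount, so editing mesh, offset, rotation or scale alone leaves existing instances unchanged.
; The event graph has no active logic.
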(fn `UserConstructionScript`
  (bind _instancedstaticmesh (`self.InstancedStaticMesh`))
  (if (!= (`self.Count`) (`self.MaxCount`))
    (`StaticMeshComponent.SetStaticMesh` _instancedstaticmesh (`self.StaticMesh_REF`))
    (`InstancedStaticMeshComponent.ClearInstances` _instancedstaticmesh)
    (for _index (range 1 (+ (`self.Count`) 1))
      (`InstancedStaticMeshComponent.AddInstance` (`self.InstancedStaticMesh`) (`KismetMathLibrary.MakeTransform` (* (- _index 0) (`self.Offset`)) (`self.Rotation`) (`self.Scale`)) false))
    (set `self.MaxCount` (`self.Count`))))