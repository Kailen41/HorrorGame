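; BP_CeilingLight is a ceiling light actor with a switchable spot light and an optional flicker.
; On BeginPlay, ShouldFlicker applies a flickering light function material to the spot light.
; ToggleLight uses a FlipFlop, first call on, to alternate spot intensity between LightIntensity and zero, swapping one mesh material slot between emissive and glass to match.
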(event `self.ReceiveBeginPlay`
  (if (`self.ShouldFlicker?`)
    (`LightComponent.SetLightFunctionMaterial` (`self.SpotLight`) "/Game/_Main/Materials/CreatedMaterials/MI_FlickeringLight.MI_FlickeringLight")))

(event `ToggleLight`
  (`/Engine/EditorBlueprintResources/StandardMacros.FlipFlop`
    (:`A`
      (`LightComponent.SetIntensity` (`self.SpotLight`) (`self.LightIntensity`))
      (`PrimitiveComponent.SetMaterial` (`self.Ceiling_Light`) 4 "/Game/_Main/Materials/CreatedMaterials/MI_Emissive.MI_Emissive"))
    (:`B`
      (`LightComponent.SetIntensity` (`self.SpotLight`) 0.0)
      (`PrimitiveComponent.SetMaterial` (`self.Ceiling_Light`) 4 "/Game/StarterContent/Materials/M_Glass.M_Glass"))))

(fn `UserConstructionScript`)