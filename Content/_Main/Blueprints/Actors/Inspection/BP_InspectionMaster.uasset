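; Base actor for inspectable items, which the player can examine up close and rotate.
; Interact moves input from the character to the item, attaches it to the character, disables collision, places it ahead of the camera and shows a name/description widget.
; Holding left mouse rotates it with mouse movement.
; IA_Interact ends inspection by returning input, applying the saved mesh transform to the actor, detaching, restoring collision and removing the widget.
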(event `/Game/_Main/Blueprints/Interfaces/I_Interaction.Interact`
  (params (FPSCharacter :type "/Game/_Main/Blueprints/BP_FPSCharacter Object Reference"))
  (bind _output_get (set `self.FPSCharacter_REF` FPSCharacter))
  (`/Game/_Main/Blueprints/BP_FPSCharacter.InspectedItem` _output_get
    (:`then`)
    (:`else`
      (`self.f_InspectItem`))))

(event `EnhancedInput|/Game/_Main/Input/InputActions/IA_Interact`
  (params (ActionValue :type Boolean) (ElapsedSeconds :type "Float (double-precision)") (TriggeredSeconds :type "Float (double-precision)") (InputAction :type "InputAction Object Reference" :default "/Game/_Main/Input/InputActions/IA_Interact.IA_Interact"))
  (:`Started`
    (`self.f_StopInspectingItem`)))

(event `Key|LeftMouseButton`
  (params (Key :type "Key Structure"))
  ;[1 0 1] Handles Rotation of inspected item
  (:`Pressed`
    (set `self.CanRotate?` true))
  (:`Released`
    (set `self.CanRotate?` false)))

(event `InputAxisKey|MouseX`
  (params (AxisValue :type "Float (single-precision)"))
  ;[1 0 1] Handles Rotation of inspected item
  (if (`self.CanRotate?`)
    (`self.K2_SetActorRotation` (`KismetMathLibrary.ComposeRotators` (`self.K2_GetActorRotation`) (`KismetMathLibrary.MakeRotator` 0.0 0.0 (* AxisValue 2.0))))))

(event `InputAxisKey|MouseY`
  (params (AxisValue :type "Float (single-precision)"))
  ;[1 0 1] Handles Rotation of inspected item
  (if (`self.CanRotate?`)
    (`self.K2_SetActorRotation` (`KismetMathLibrary.ComposeRotators` (`self.K2_GetActorRotation`) (`KismetMathLibrary.MakeRotator` 0.0 (* AxisValue 2.0))))))

(fn `f_InspectItem`
  (bind _returnvalue (`GameplayStatics.GetPlayerController` 0))
  (bind _fpscharacter_ref (`self.FPSCharacter_REF`))
  (bind (_iteminformation_itemname _iteminformation_itemdescription) (break `/Game/_Main/Blueprints/Structs/S_ItemInformation` (`self.ItemInformation`)))
  (set `self.ItemOriginalLocation` (`SceneComponent.RelativeLocation` (`self.StaticMesh`)))
  (set `self.ItemOriginalRotation` (`SceneComponent.RelativeRotation` (`self.StaticMesh`)))
  (`self.DisableInput` _fpscharacter_ref _returnvalue)
  (`self.EnableInput` _returnvalue)
  (`self.K2_AttachToComponent` (`/Game/_Main/Blueprints/BP_FPSCharacter.Item` _fpscharacter_ref) "None" "SnapToTarget" "SnapToTarget" "KeepRelative")
  (`PrimitiveComponent.SetCollisionEnabled` (`self.StaticMesh`) "NoCollision")
  (set `/Game/_Main/Blueprints/BP_FPSCharacter.InspectedItem` self (`self.FPSCharacter_REF`))
  (bind _offsetlocation (`self.f_ItemInspectionCameraOffset`))
  (`self.K2_SetActorLocation` _offsetlocation)
  (bind _returnvalue_2 (`|CreateWidget` "/Game/_Main/Blueprints/UMG/W_ItemInformationDisplay.W_ItemInformationDisplay_C" null _iteminformation_itemname _iteminformation_itemdescription))
  (bind _output_get (set `self.ItemUI_REF` _returnvalue_2))
  (`UserWidget.AddToViewport` _output_get 0))

(fn `f_ItemInspectionCameraOffset`
  (returns (OffsetLocation :type "Vector Structure"))
  (bind _returnvalue (`GameplayStatics.GetPlayerCameraManager` 0))
  (return (+ (`PlayerCameraManager.GetCameraLocation` _returnvalue) (* (`KismetMathLibrary.GetForwardVector` (`PlayerCameraManager.GetCameraRotation` _returnvalue)) (`self.InspectionDistance`)))))

(fn `f_StopInspectingItem`
  (bind _returnvalue (`GameplayStatics.GetPlayerController` 0))
  (bind _itemui_ref (`self.ItemUI_REF`))
  (`self.DisableInput` _returnvalue)
  (`self.EnableInput` (`self.FPSCharacter_REF`) _returnvalue)
  (`self.K2_SetActorRelativeLocation` (`self.ItemOriginalLocation`))
  (`self.K2_SetActorRelativeRotation` (`self.ItemOriginalRotation`))
  (`self.K2_DetachFromActor` "KeepRelative")
  (`PrimitiveComponent.SetCollisionEnabled` (`self.StaticMesh`) "QueryAndPhysics")
  (`/Engine/EditorBlueprintResources/StandardMacros.IsValid` _itemui_ref
    (:`Is Valid`
      (`Widget.RemoveFromParent` _itemui_ref))))

(fn `UserConstructionScript`)